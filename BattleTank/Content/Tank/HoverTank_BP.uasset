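; HoverTank_BP is a player-controllable tank that delegates aiming, firing and movement to its TankAiming and TankMovement components.
; BeginPlay hands the barrel and turret to TankAiming and the left and right tracks to TankMovement.
; Aim axes rotate the camera rig, split into yaw on AzimuthGimbal and pitch on SpringArm.
; Movement axes feed forward and turn requests to TankMovement, and Fire triggers TankAiming.
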(event `self.ReceiveBeginPlay`
  (`TankAimingComponent.Initialize` (`self.TankAiming`) (`self.TankBarrel`) (`self.TankTurret`))
  (`TankMovementComponent.Initialize` (`self.TankMovement`) (`self.LeftTrack`) (`self.RightTrack`)))

(event `InputAxis|AimAzimuth`
  (params (AxisValue :type "Float (single-precision)"))
  ;[1 1 1] Setup aim input
  (`SceneComponent.K2_AddLocalRotation` (`self.AzimuthGimbal`) (`KismetMathLibrary.MakeRotator` 0.0 0.0 AxisValue) false false))

(event `InputAxis|AimElevation`
  (params (AxisValue :type "Float (single-precision)"))
  ;[1 1 1] Setup aim input
  (`SceneComponent.K2_AddLocalRotation` (`self.SpringArm`) (`KismetMathLibrary.MakeRotator` 0.0 AxisValue) false false))

(event `InputAxis|MoveForward`
  (params (AxisValue :type "Float (single-precision)"))
  ;[1 1 1] Setup movement input
  (`TankMovementComponent.WishForward` (`self.TankMovement`) AxisValue))

(event `InputAxis|MoveTurn`
  (params (AxisValue :type "Float (single-precision)"))
  ;[1 1 1] Setup movement input
  (`TankMovementComponent.WishTurn` (`self.TankMovement`) AxisValue))

(event `InputAction|Fire`
  (params (Key :type "Key Structure"))
  ;[1 1 1] Setup aim input
  (:`Pressed`
    (`TankAimingComponent.Fire` (`self.TankAiming`))))

(fn `UserConstructionScript`)